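; BP_Player is the player Blueprint, handling movement and mouse look through Enhanced Input actions.
; Movement actions feed AddMovementInput along forward and right vectors from the full control rotation, with left/right input negated.
; Mouse actions feed controller yaw and pitch, with pitch inverted, so looking around steers the movement direction.
; The construction script is empty.
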(event `EnhancedInput|/Game/Input_Actions/IA_ForwardBackward`
  (params (ActionValue :type "Float (double-precision)") (ElapsedSeconds :type "Float (double-precision)") (TriggeredSeconds :type "Float (double-precision)") (InputAction :type "InputAction Object Reference" :default "/Game/Input_Actions/IA_ForwardBackward.IA_ForwardBackward"))
  (:`Triggered`
    (`self.AddMovementInput` (`KismetMathLibrary.GetForwardVector` (`self.GetControlRotation`)) ActionValue)))

(event `EnhancedInput|/Game/Input_Actions/IA_LeftRight`
  (params (ActionValue :type "Float (double-precision)") (ElapsedSeconds :type "Float (double-precision)") (TriggeredSeconds :type "Float (double-precision)") (InputAction :type "InputAction Object Reference" :default "/Game/Input_Actions/IA_LeftRight.IA_LeftRight"))
  (:`Triggered`
    (`self.AddMovementInput` (`KismetMathLibrary.GetRightVector` (`self.GetControlRotation`)) (* ActionValue -1.0))))

(event `EnhancedInput|/Game/Input_Actions/IA_MouseUpDown`
  (params (ActionValue :type "Float (double-precision)") (ElapsedSeconds :type "Float (double-precision)") (TriggeredSeconds :type "Float (double-precision)") (InputAction :type "InputAction Object Reference" :default "/Game/Input_Actions/IA_MouseUpDown.IA_MouseUpDown"))
  (:`Triggered`
    (`self.AddControllerPitchInput` (* ActionValue -1.0))))

(event `EnhancedInput|/Game/Input_Actions/IA_MouseLeftRight`
  (params (ActionValue :type "Float (double-precision)") (ElapsedSeconds :type "Float (double-precision)") (TriggeredSeconds :type "Float (double-precision)") (InputAction :type "InputAction Object Reference" :default "/Game/Input_Actions/IA_MouseLeftRight.IA_MouseLeftRight"))
  (:`Triggered`
    (`self.AddControllerYawInput` ActionValue)))

(fn `UserConstructionScript`)